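; Base character Blueprint providing stats, health, hunger, inventory listing and surface-based footstep sounds.
; On BeginPlay, it maps Strength, Endurance and Agility tiers through DT_Stats to carry weight, health and walk speed.
; A self-rescheduling HungerTick, not started here, drains hunger and applies starvation damage at zero, while death only prints a message.
; Interact prints inventory items, and footsteps look up sounds by physical material with a concrete fallback.
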(event OnComponentEndOverlap(ItemContainerCollider)
  (params (OverlappedComponent :type Primitive%20Component%20Object%20Reference) (OtherActor :type Actor%20Object%20Reference) (OtherComp :type Primitive%20Component%20Object%20Reference) (OtherBodyIndex :type Integer)))

(event Custom|Die
  (Development|PrintString (Utilities|String|Append (Utilities|GetDisplayName self) " Is Dead!")))

(event Custom|HungerTick
  (bind _result (Math|Integer|DecrementInt (Variables|Stats|GetHunger))
    (:%20%20
      (if (<= _result 0)
        (Variables|Stats|SetHunger 0)
        (CallFunction|Damage (Variables|Settings|GetStarveHealthPenalty)))
      (Utilities|FlowControl|Delay (Variables|Settings|GetHungerTickRate))
      (CallFunction|HungerTick))))

(event EventBeginPlay
  (CallFunction|CalculateStats))

(event EventDamage
  (params (Amount :type Integer))
  (Variables|Stats|SetHealth (- (Variables|Stats|GetHealth) Amount))
  (if (<= (Variables|Stats|GetHealth) 0)
    (CallFunction|Die)))

(event EventInteract
  (params (CallingActor :type Actor%20Object%20Reference))
  (bind _bp_inventorycomponent (Variables|Default|GetBP_InventoryComponent))
  (bind _items (Variables|/Game/Blueprints/Character/BP_InventoryComponent.BP_InventoryComponent_C|GetItems _bp_inventorycomponent))
  (if (> (Utilities|Array|Length _items) 0)
    (Development|PrintString "---------------" true true "(R=1.000000,G=0.000000,B=0.627451,A=1.000000)")
    (for _array_element _items
      (Development|PrintString (Variables|/Game/Items/ItemBase.ItemBase_C|GetName _array_element) true true "(R=1.000000,G=0.000000,B=0.627451,A=1.000000)"))
    (Development|PrintString "---------------" true true "(R=1.000000,G=0.000000,B=0.627451,A=1.000000)")
    (else
      (Development|PrintString (Utilities|String|Append (Utilities|GetDisplayName self) " Has No Items") true true "(R=1.000000,G=0.000000,B=0.627451,A=1.000000)" 2.0 "CItems"))))

(fn ConstructionScript)

(fn CalculateStats
  (bind _bp_statscomponent (Variables|Default|GetBP_StatsComponent))
  (Utilities|FlowControl|Sequence
    (:then_0
      (bind _returnvalue (Utilities|GetDataTableRow "/Game/Blueprints/Character/DT_Stats.DT_Stats" "Strength")
        (:then
          (switch Utilities|FlowControl|Switch|SwitchonEN_StatLevel (Variables|/Game/Blueprints/Character/BP_StatsComponent.BP_StatsComponent_C|GetStrength _bp_statscomponent)
            (:NewEnumerator0
              (Variables|Stats|SetCarryWeight (.poormodifier _returnvalue)))
            (:NewEnumerator1
              (Variables|Stats|SetCarryWeight (.averagemodifier _returnvalue)))
            (:NewEnumerator2
              (Variables|Stats|SetCarryWeight (.goodmodifier _returnvalue)))))))
    (:then_1
      (bind _returnvalue_2 (Utilities|GetDataTableRow "/Game/Blueprints/Character/DT_Stats.DT_Stats" "Endurance")
        (:then
          (switch Utilities|FlowControl|Switch|SwitchonEN_StatLevel (Variables|/Game/Blueprints/Character/BP_StatsComponent.BP_StatsComponent_C|GetEndurance _bp_statscomponent)
            (:NewEnumerator0
              (bind _output_get (Variables|Stats|SetHealth (Math|Float|Truncate (.poormodifier _returnvalue_2))))
              (Variables|Stats|SetMaxHealth _output_get))
            (:NewEnumerator1
              (bind _output_get_2 (Variables|Stats|SetHealth (Math|Float|Truncate (.averagemodifier _returnvalue_2))))
              (Variables|Stats|SetMaxHealth _output_get_2))
            (:NewEnumerator2
              (bind _output_get_3 (Variables|Stats|SetHealth (Math|Float|Truncate (.goodmodifier _returnvalue_2))))
              (Variables|Stats|SetMaxHealth _output_get_3))))))
    (:then_2
      (bind _returnvalue_3 (Utilities|GetDataTableRow "/Game/Blueprints/Character/DT_Stats.DT_Stats" "Agility")
        (:then
          (switch Utilities|FlowControl|Switch|SwitchonEN_StatLevel (Variables|/Game/Blueprints/Character/BP_StatsComponent.BP_StatsComponent_C|GetAgility _bp_statscomponent)
            (:NewEnumerator0
              (Variables|Stats|SetMoveSpeed (.poormodifier _returnvalue_3)))
            (:NewEnumerator1
              (Variables|Stats|SetMoveSpeed (.averagemodifier _returnvalue_3)))
            (:NewEnumerator2
              (Variables|Stats|SetMoveSpeed (.goodmodifier _returnvalue_3))))
          (Variables|/Script/Engine.CharacterMovementComponent|SetMaxWalkSpeed (Variables|Character|GetCharacterMovement) (Variables|Stats|GetMoveSpeed)))))))

(fn AddHunger
  (params (Value :type Integer))
  (bind _output_get (Variables|Stats|SetHunger (+ Value (Variables|Stats|GetHunger))))
  (if (>= _output_get 100)
    (bind _output_get_2 (Variables|Stats|SetHunger 100)))
  (Development|PrintString (Utilities|String|Append "Your hunger is now " (Utilities|String|ToString(Integer) _output_get_2))))

(fn GetHealthPercentage
  (return (/ (Math|Conversions|ToFloat(Integer) (Variables|Stats|GetHealth)) (Math|Conversions|ToFloat(Integer) (Variables|Stats|GetMaxHealth)))))

(fn GetHungerPercentage
  (return (/ (Math|Conversions|ToFloat(Integer) (Variables|Stats|GetHunger)) 1e+02)))

(fn PlayFootstepSound
  (params (PhysMat :type Physical%20Material%20Object%20Reference) (Location :type Vector))
  (bind _materialfootstep (Variables|Default|GetMaterialFootstep))
  (bind (_value _returnvalue) (Utilities|Map|Find _materialfootstep PhysMat))
  (if _returnvalue
    (Audio|PlaySoundatLocation _value Location "0, 0, 0" 1.0 1.0 0.0 0 0 0 0)
    (else
      (Audio|PlaySoundatLocation "/Game/Sounds/Footsteps/SC_FootstepsConcrete.SC_FootstepsConcrete" Location "0, 0, 0" 1.0 1.0 0.0 0 0 0 0))))