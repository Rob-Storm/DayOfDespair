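; BP_NPC is an AI-controlled character that toggles following the player when interacted with.
; Interact casts its controller to BP_AI_Controller and inverts that controller's FollowPlayer flag; the branch that then checks the flag leads nowhere.
; UpdateWalkSpeed sets the movement component's max walk speed, with no caller in this Blueprint.
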(event EventBeginPlay
  (|CallParentFunction) ; This node is disabled and will not be called.\nDrag off pins to build functionality.
)

(event Collision|EventActorBeginOverlap
  (params (OtherActor :type Actor%20Object%20Reference)))

(event EventTick
  (params (DeltaSeconds :type Float%20%28single-precision%29)))

(event EventInteract
  (params (CallingActor :type Actor%20Object%20Reference))
  (bind _asbp_ai_controller (Utilities|Casting|CastToBP_AI_Controller (Pawn|GetController)))
  (Default|SetFollowPlayer _asbp_ai_controller (CallFunction|InvertBool (Variables|/Game/AI/BP_AI_Controller.BP_AI_Controller_C|GetFollowPlayer? _asbp_ai_controller)))
  (if (Variables|/Game/AI/BP_AI_Controller.BP_AI_Controller_C|GetFollowPlayer? _asbp_ai_controller)
    _))

(fn ConstructionScript
  (|CallParentFunction))

(fn UpdateWalkSpeed
  (params (NewWalkSpeed :type Float%20%28double-precision%29))
  (Variables|/Script/Engine.CharacterMovementComponent|SetMaxWalkSpeed (Variables|Character|GetCharacterMovement) NewWalkSpeed))