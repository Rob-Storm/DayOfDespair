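; BP_StatsComponent is a character stats component that holds randomly rolled Strength, Endurance and Agility values.
; On BeginPlay, GenerateStats sets each stat independently to one of three enum values through GetRandomStat.
; GetStats returns the values as an array, while GetStatsFormatted returns a map keyed by stat name.
; PrintStats uses that map to print each name and value on screen for debugging.
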(event EventBeginPlay
  (Stats|GenerateStats))

(fn GetRandomStat
  (switch int (Math|Random|RandomIntegerinRange 0 2)
    (:0
      (return "NewEnumerator0"))
    (:1
      (return "NewEnumerator1"))
    (:2
      (return "NewEnumerator2"))))

(fn GetStats
  (return (Utilities|Array|MakeArray (Variables|Stats|GetStrength) (Variables|Stats|GetEndurance) (Variables|Stats|GetAgility))))

(fn GetStatsFormatted
  (return (Utilities|Map|MakeMap (Utilities|String|MakeLiteralString "Strength") (Variables|Stats|GetStrength) (Utilities|String|MakeLiteralString "Endurance") (Variables|Stats|GetEndurance) (Utilities|String|MakeLiteralString "Agility") (Variables|Stats|GetAgility))))

(fn GenerateStats
  (Variables|Stats|SetStrength (Stats|GetRandomStat))
  (Variables|Stats|SetEndurance (Stats|GetRandomStat))
  (Variables|Stats|SetAgility (Stats|GetRandomStat)))

(fn PrintStats
  (bind _newparam (Stats|GetStatsFormatted))
  (bind _keys (Utilities|Map|Keys _newparam))
  (for (_array_element _array_index) _keys
    (bind _values (Utilities|Map|Values _newparam))
    (Development|PrintString (Utilities|String|Append _array_element ", " (Utilities|String|EnumtoString (Utilities|Array|Get(acopy) _values _array_index))) true true "(R=0.670580,G=1.000000,B=0.000000,A=1.000000)")))