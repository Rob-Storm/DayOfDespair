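; BP_ItemBase is a base world item actor that characters pick up into their inventory.
; The construction script sets the WorldModel mesh from the item's ItemData.
; On Interact, it casts the caller to BP_CharacterBase, adds ItemData to that character's BPInventoryComponent if CanAddItem allows, then destroys itself.
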(event EventInteract
  (params (CallingActor :type Actor%20Object%20Reference))
  (bind _itemdata (Variables|Default|GetItemData))
  (bind _asbp_character_base (Utilities|Casting|CastToBP_CharacterBase CallingActor))
  (if (Default|CanAddItem (Variables|/Game/Blueprints/Character/BP_CharacterBase.BP_CharacterBase_C|GetBP_InventoryComponent _asbp_character_base) _itemdata)
    (Default|AddItem (Variables|/Game/Blueprints/Character/BP_CharacterBase.BP_CharacterBase_C|GetBP_InventoryComponent _asbp_character_base) _itemdata)
    (Actor|DestroyActor)))

(fn ConstructionScript
  (Components|StaticMesh|SetStaticMesh (Variables|Default|GetWorldModel) (Variables|/Game/Items/DA_ItemBase.DA_ItemBase_C|GetModel (Variables|Default|GetItemData))))