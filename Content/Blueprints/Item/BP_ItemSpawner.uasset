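; BP_ItemSpawner is a placeable actor that spawns a random item at its own location when play begins.
; It picks a random entry from ItemSpawnGroup and passes it as ItemData to a newly spawned BP_ItemActor at unit scale.
; The item takes either a random Z rotation or the spawner's rotation, depending on RandomZRotation.
; An empty group spawns nothing and prints a red on-screen warning naming the spawner.
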(event EventBeginPlay
  (bind _itemspawngroup (Variables|SpawnSettings|GetItemSpawnGroup))
  (if (> (Utilities|Array|Length _itemspawngroup) 0)
    (if (Variables|SpawnSettings|GetRandomZRotation)
      (Variables|Default|SetspawnRotation (Math|Rotator|MakeRotator 0.0 0.0 (Math|Random|RandomFloatinRange 0.0 3.6e+02)))
      (else
        (Variables|Default|SetspawnRotation (Transformation|GetActorRotation))))
    (Game|SpawnActorfromClass "/Game/Blueprints/Item/BP_ItemActor.BP_ItemActor_C" (Math|Transform|MakeTransform (Transformation|GetActorLocation) (Variables|Default|GetspawnRotation)) "Undefined" "MultiplyWithRoot" 0 (.OutItem (Utilities|Array|Random _itemspawngroup)) 0)
    (else
      (Development|PrintString (Utilities|String|Append (Utilities|GetDisplayName self) " Has empty spawn group") true true "(R=1.000000,G=0.000000,B=0.000000,A=1.000000)" 1e+01))))

(fn ConstructionScript)