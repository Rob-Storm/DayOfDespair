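; BP_ContainerPrefab is a configurable item container that opens an inventory screen when interacted with.
; Its construction script applies the chosen model to the mesh and passes the carry weight limit to its container component.
; On Interact, it creates a container inventory widget bound to itself, adds it to the viewport and hands UI control to it through the BP_PC_DoD player controller.
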(event EventBeginPlay)

(event Collision|EventActorBeginOverlap
  (params (OtherActor :type Actor%20Object%20Reference)))

(event EventTick
  (params (DeltaSeconds :type Float%20%28single-precision%29)))

(event EventInteract
  (params (CallingActor :type Actor%20Object%20Reference))
  (bind _returnvalue (Game|GetPlayerController 0))
  (bind _returnvalue_2 (UserInterface|CreateWidget "/Game/Blueprints/Widgets/Container/WBP_ContainerInventory.WBP_ContainerInventory_C" _returnvalue self))
  (UserInterface|Viewport|AddtoViewport _returnvalue_2 0)
  (bind _asbp_pc_do_d (Utilities|Casting|CastToBP_PC_DoD _returnvalue))
  (Default|SetUIControl _asbp_pc_do_d _returnvalue_2))

(fn ConstructionScript
  (Components|StaticMesh|SetStaticMesh (Variables|Default|GetContainerModel) (Variables|Container|GetModel))
  (Variables|/Game/Blueprints/Item/BP_ContainerComponent.BP_ContainerComponent_C|SetMaxCarryWeight (Variables|Default|GetBP_ContainerComponent) (Variables|Container|GetMaxCarryWeight)))