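; BP_ItemActor is a world item that characters can pick up and use, with its mesh and behavior driven by an ItemData reference.
; The construction script sets the mesh from ItemData.
; Interact accepts only BP_CharacterBase callers, adds the data to their inventory component if it can be added, then destroys the actor.
; Use delegates to ItemData's UseItem and plays its use sound in 2D.
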(event EventUse
  (params (CallingCharacter :type BP%20Character%20Base%20Object%20Reference))
  (bind _itemdata (Variables|Item|GetItemData))
  (Default|UseItem _itemdata CallingCharacter)
  (Audio|PlaySound2D (Variables|/Game/Items/ItemBase.ItemBase_C|GetUseSound _itemdata) 1.0 1.0 0.0 0 0))

(event EventInteract
  (params (CallingActor :type Actor%20Object%20Reference))
  (bind _asbp_character_base (Utilities|Casting|CastToBP_CharacterBase CallingActor))
  (if (Default|CanAddItem (Variables|/Game/Blueprints/Character/BP_CharacterBase.BP_CharacterBase_C|GetBP_InventoryComponent _asbp_character_base) (Variables|Item|GetItemData))
    (Default|AddItem (Variables|/Game/Blueprints/Character/BP_CharacterBase.BP_CharacterBase_C|GetBP_InventoryComponent _asbp_character_base) (Variables|Item|GetItemData))
    (Actor|DestroyActor)))

(fn ConstructionScript
  (Components|StaticMesh|SetStaticMesh (Variables|Default|GetItemModel) (Variables|/Game/Items/ItemBase.ItemBase_C|GetModel (Variables|Item|GetItemData))))