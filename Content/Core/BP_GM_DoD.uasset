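; Game mode that runs a day/night clock, counting minutes and days and crossfading ambient sound by time of day.
; A self-calling TimeTick event advances time after each configurable delay, prints a 12-hour readout and broadcasts OnTimeTick.
; AmbientCheck listens to that dispatcher and swaps morning, noon and night audio components at fixed minutes.
; GetSunAngleFromTime converts minutes into sun pitch but is not called here.
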(event Custom|TimeTick
  (if (== (Variables|Default|GetCurrentTime) 1439)
    (Variables|Default|SetCurrentTime 0)
    (Math|Integer|IncrementInt (Variables|Default|GetDay)
      (:%20%20
        _))
    (else
      (Math|Integer|IncrementInt (Variables|Default|GetCurrentTime)
        (:%20%20
          _))))
  (Development|PrintString (Utilities|String|Append "Day: " (Utilities|String|ToString(Integer) (Variables|Default|GetDay)) " | " (CallFunction|GetTimeFormatted)) true true "(R=1.000000,G=1.000000,B=1.000000,A=1.000000)" 2.0 "Time")
  (Utilities|FlowControl|Delay (Variables|Default|GetTimeTickDelay))
  (CallFunction|TimeTick)
  (Default|CallOnTimeTick (Variables|Default|GetCurrentTime)))

(event Custom|AmbientCheck
  (params (CurrentTime :type Integer))
  (if (== CurrentTime 345)
    (Audio|Components|Audio|FadeOut (Variables|Default|GetNightSound) 5.0 0.0 "Linear" :!class /Script/Engine.AudioComponent)
    (Audio|Components|Audio|FadeIn (Variables|Default|GetMorningSound) 5.0 1.0 0.0 "Linear" :!class /Script/Engine.AudioComponent)
    (Development|PrintString "Morning" true true "(R=1.000000,G=1.000000,B=1.000000,A=1.000000)" 2.0 "TimeOfDay")
    (elif (== CurrentTime 600)
      (Audio|Components|Audio|FadeOut (Variables|Default|GetMorningSound) 5.0 0.0 "Linear" :!class /Script/Engine.AudioComponent)
      (Audio|Components|Audio|FadeIn (Variables|Default|GetNoonSound) 5.0 1.0 0.0 "Linear" :!class /Script/Engine.AudioComponent)
      (Development|PrintString "Noon" true true "(R=1.000000,G=1.000000,B=1.000000,A=1.000000)" 2.0 "TimeOfDay")
      (elif (== CurrentTime 1050)
        (Audio|Components|Audio|FadeOut (Variables|Default|GetNoonSound) 5.0 0.0 "Linear" :!class /Script/Engine.AudioComponent)
        (Audio|Components|Audio|FadeIn (Variables|Default|GetNightSound) 5.0 1.0 0.0 "Linear" :!class /Script/Engine.AudioComponent)
        (Development|PrintString "Night" true true "(R=1.000000,G=1.000000,B=1.000000,A=1.000000)" 2.0 "TimeOfDay")))))

(event EventBeginPlay
  (CallFunction|TimeTick)
  (EventDispatchers|BindEventtoOnTimeTick (delegate Custom|AmbientCheck))
  (Audio|Components|Audio|FadeIn (Variables|Default|GetMorningSound) 2.0 1.0 0.0 "Linear" :!class /Script/Engine.AudioComponent))

(fn ConstructionScript
  (Audio|Components|Audio|SetSound (Variables|Default|GetMorningSound) (Variables|Ambience|GetMorningAmbience))
  (Audio|Components|Audio|SetSound (Variables|Default|GetNoonSound) (Variables|Ambience|GetNoonAmbience))
  (Audio|Components|Audio|SetSound (Variables|Default|GetNightSound) (Variables|Ambience|GetNightAmbience)))

(fn GetTimeFormatted
  (bind _currenttime (Variables|Default|GetCurrentTime))
  (bind _currenttime_2 (Variables|Default|GetCurrentTime))
  (bind _returnvalue (Math|Conversions|ToFloat(Integer) _currenttime_2))
  (bind (_remainder _returnvalue_2) (Math|Float|Division(WholeandRemainder) _returnvalue 6e+01))
  (LocalVariables|SetHour _returnvalue_2)
  (if (> (LocalVariables|GetHour) 12)
    (LocalVariables|SetHour (- (LocalVariables|GetHour) 12)))
  (LocalVariables|SetMinute (Math|Float|Truncate _remainder))
  (if (and (>= _currenttime 720) (<= _currenttime 1439))
    (LocalVariables|SetPeriodString "PM")
    (else
      (LocalVariables|SetPeriodString "AM")))
  (if (== (LocalVariables|GetHour) 0)
    (LocalVariables|SetHourString "12")
    (else
      (LocalVariables|SetHourString (Utilities|String|ToString(Integer) (LocalVariables|GetHour)))))
  (if (< (LocalVariables|GetMinute) 10)
    (LocalVariables|SetMinuteString (Utilities|String|Append "0" (Utilities|String|ToString(Integer) (LocalVariables|GetMinute))))
    (else
      (LocalVariables|SetMinuteString (Utilities|String|ToString(Integer) (LocalVariables|GetMinute)))))
  (return (Utilities|String|Append (LocalVariables|GetHourString) " : " (LocalVariables|GetMinuteString) " " (LocalVariables|GetPeriodString))))

(fn GetSunAnglefromTime
  (params (New%20Time :type Integer))
  (return (Math|Rotator|MakeRotator 0.0 (- (* New%20Time 0.25) 2.7e+02) 0.0)))