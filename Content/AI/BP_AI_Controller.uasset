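; AI controller that runs the default character behavior tree and feeds it what it sees of the player.
; Perception updates are filtered to sight stimuli on player character 0, which set or clear the TargetActor blackboard key.
; When sight is lost, the stimulus location is saved as LastKnownLocation.
; A DoOnce is triggered on sighting and reset on loss, with nothing wired after it.
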(event OnTargetPerceptionUpdated(AIPerception)
  (params (Actor :type Actor%20Object%20Reference) (Stimulus :type AI%20Stimulus%20Structure))
  (CallFunction|HandleSightSense Actor Stimulus))

(event EventBeginPlay
  (AI|RunBehaviorTree "/Game/AI/BT_CharacterDefault.BT_CharacterDefault"))

(fn ConstructionScript)

(fn HandleSightSense
  (params (Actor :type Actor%20Object%20Reference) (Stimulus :type AI%20Stimulus%20Structure))
  (bind _returnvalue (Class|AIPerceptionSystem|GetSenseClassforStimulus Stimulus))
  (if (== _returnvalue "/Script/AIModule.AISense_Sight")
    (if (== Actor (Game|GetPlayerCharacter 0))
      (AI|Components|Blackboard|SetValueasObject (Variables|Default|GetBlackboard) (Utilities|Name|MakeLiteralName "TargetActor") (Utilities|SelectObject (Game|GetPlayerCharacter 0) 0 (.bsuccessfullysensed Stimulus)))
      (if (.bsuccessfullysensed Stimulus)
        (Utilities|FlowControl|DoOnce false :!label _label)
        (else
          (AI|Components|Blackboard|SetValueasVector (Variables|Default|GetBlackboard) (Utilities|Name|MakeLiteralName "LastKnownLocation") (.stimuluslocation Stimulus))
          (goto _label Reset)))
      (else
        (return)))
    (else
      (return))))